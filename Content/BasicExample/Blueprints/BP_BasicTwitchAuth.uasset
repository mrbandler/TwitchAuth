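; BP_BasicTwitchAuth is a basic example of Twitch sign-in and channel subscription checking.
; On BeginPlay it binds the sign-in and subscription callbacks, then starts user sign-in.
; A successful sign-in stores and prints the Twitch user, then checks their subscription to ChannelToCheck.
; The subscription callback prints the subscribed channel, and negative results in either callback print the last error message.
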(event Custom|OnUserSignedInEvent
  (params (SignedIn :type Boolean))
  (if SignedIn
    (bind _returnvalue (Class|TwitchAuthActor|GetSignedinTwitchUser))
    (bind _output_get (Variables|Default|SetTwitchUser _returnvalue))
    (Development|PrintString (Utilities|String|Append (.display_name (Utilities|Struct|BreakTwitchUser _output_get)) " just signed in!") true true "(R=0.091889,G=1.000000,B=0.000000,A=1.000000)" 5.0)
    (Class|TwitchAuthActor|IsTwitchUserSubscribedtoChannel (Variables|Default|GetTwitchUser) (Variables|Default|GetChannelToCheck))
    (else
      (bind _returnvalue_2 (Class|TwitchAuthActor|GetLastError))
      (Development|PrintString (.message _returnvalue_2) true true "(R=1.000000,G=0.000000,B=0.052997,A=1.000000)" 5.0))))

(event Custom|OnTwitchUserSubscribedToChannelEvent
  (params (bSubscribed :type Boolean) (TwitchSubscription :type Twitch%20Subscription%20Structure))
  (if bSubscribed
    (Development|PrintString (Utilities|String|Append (.display_name (Utilities|Struct|BreakTwitchUser (Variables|Default|GetTwitchUser))) " is subscribed to the channel " (.name (Utilities|Struct|BreakTwitchChannel (.channel (Utilities|Struct|BreakTwitchSubscription TwitchSubscription))))) true true "(R=0.032664,G=1.000000,B=0.000000,A=1.000000)" 5.0)
    (else
      (bind _returnvalue (Class|TwitchAuthActor|GetLastError))
      (Development|PrintString (.message _returnvalue) true true "(R=1.000000,G=0.000000,B=0.052997,A=1.000000)" 5.0))))

(event EventBeginPlay
  (EventDispatchers|AssignOnUserSignedin (delegate Custom|OnUserSignedInEvent))
  (EventDispatchers|BindEventtoOnTwitchUserSubscribedtoChannel (delegate Custom|OnTwitchUserSubscribedToChannelEvent))
  (Class|TwitchAuthActor|StartUserSignin))

(fn ConstructionScript)