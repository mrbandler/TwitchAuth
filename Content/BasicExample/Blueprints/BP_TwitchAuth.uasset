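; Example actor that signs a user into Twitch through an in-game web browser widget and checks their channel relationship.
; On BeginPlay it creates the browser widget and passes it to TwitchAuth, whose page-load events toggle browser and cursor visibility.
; Result events chain authentication, subscription and follow checks against a hardcoded channel, printing results or errors.
; The follow check runs only for subscribers, and its handler always takes the success branch.
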(event OnUserAuthenticated(TwitchAuth)
  (params (bAuthenticated :type Boolean))
  (if bAuthenticated
    (Development|PrintString (Utilities|String|Append (.display_name (Utilities|Struct|BreakTwitchUser (Class|TwitchAuthComponent|GetUser (Variables|Default|GetTwitchAuth)))) " just signed in!") true true "(R=0.071240,G=1.000000,B=0.000000,A=1.000000)" 5.0)
    (Class|TwitchAuthComponent|IsUserSubscribedtoChannel (Variables|Default|GetTwitchAuth) "wheeze202")
    (else
      (TwitchAuth|PrintTwitchError (Class|TwitchAuthComponent|GetLastError (Variables|Default|GetTwitchAuth))))))

(event OnUserSubscribedtoChannel(TwitchAuth)
  (params (bSubscribed :type Boolean) (TwitchSubscription :type Twitch%20Subscription%20Structure))
  (if bSubscribed
    (Development|PrintString (Utilities|String|Append (.display_name (Utilities|Struct|BreakTwitchUser (Class|TwitchAuthComponent|GetUser (Variables|Default|GetTwitchAuth)))) " is subscribed to " (.name (Utilities|Struct|BreakTwitchChannel (.channel (Utilities|Struct|BreakTwitchSubscription TwitchSubscription))))) true true "(R=0.105615,G=1.000000,B=0.000000,A=1.000000)" 5.0)
    (Class|TwitchAuthComponent|IsUserFollowingChannel (Variables|Default|GetTwitchAuth) "wheeze202")
    (else
      (TwitchAuth|PrintTwitchError (Class|TwitchAuthComponent|GetLastError (Variables|Default|GetTwitchAuth))))))

(event OnAuthenticationPageLoaded(TwitchAuth)
  (Widget|SetVisibility (Variables|Default|GetWebBrowser) "Visible")
  (Variables|/Script/Engine.PlayerController|SetbShowMouseCursor (Game|GetPlayerController 0) true))

(event OnAccessTokenPageLoaded(TwitchAuth)
  (Widget|SetVisibility (Variables|Default|GetWebBrowser) "Hidden")
  (Variables|/Script/Engine.PlayerController|SetbShowMouseCursor (Game|GetPlayerController 0) false))

(event OnUserFollowingChannel(TwitchAuth)
  (params (bSubscribed :type Boolean) (TwitchFollow :type Twitch%20Follow%20Structure))
  (if true
    (Development|PrintString (Utilities|String|Append (.display_name (Utilities|Struct|BreakTwitchUser (Class|TwitchAuthComponent|GetUser (Variables|Default|GetTwitchAuth)))) " is following " (.name (Utilities|Struct|BreakTwitchChannel (.channel (Utilities|Struct|BreakTwitchFollow TwitchFollow))))) true true "(R=0.105615,G=1.000000,B=0.000000,A=1.000000)" 5.0)
    (else
      (TwitchAuth|PrintTwitchError (Class|TwitchAuthComponent|GetLastError (Variables|Default|GetTwitchAuth))))))

(event EventBeginPlay
  (bind _returnvalue (UserInterface|CreateWidget "/TwitchAuth/BasicExample/UMG/WBP_WebBrowserBasicExample.WBP_WebBrowserBasicExample_C" (Game|GetPlayerController 0)))
  (bind _output_get (Variables|Widgets|SetWebBrowserWidget _returnvalue))
  (Variables|Default|SetWebBrowser (Variables|/TwitchAuth/BasicExample/UMG/WBP_WebBrowserBasicExample.WBP_WebBrowserBasicExample_C|GetWebBrowser_55 _output_get))
  (UserInterface|Viewport|AddtoViewport (Variables|Widgets|GetWebBrowserWidget) 0)
  (Class|TwitchAuthComponent|Authenticate (Variables|Default|GetTwitchAuth) (Variables|Default|GetWebBrowser)))

(fn ConstructionScript)

(fn PrintTwitchError
  (params (TwitchError :type Twitch%20Error%20Structure))
  (bind (_error _status _message) (Utilities|Struct|BreakTwitchError TwitchError))
  (Development|PrintString (Utilities|String|Append _error "(" (Utilities|String|ToString(Integer) _status) "): " _message) true true "(R=1.000000,G=0.055564,B=0.000000,A=1.000000)" 5.0))