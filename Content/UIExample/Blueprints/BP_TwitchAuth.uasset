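; Example actor that signs the player into Twitch and verifies their subscription to a configured channel.
; On BeginPlay it restores the saved access token, picks the pre- or post-authentication widget, and starts TwitchAuth through the widget's web browser.
; TwitchAuth events toggle browser and cursor visibility.
; Successful sign-in saves the token and checks the subscription for the post-auth widget; failure prints the error, clears the token and retries.
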(event OnUserAuthenticated(TwitchAuth)
  (params (bAuthenticated :type Boolean))
  (TwitchAuth|OnUserAuthenticated bAuthenticated))

(event OnUserSubscribedtoChannel(TwitchAuth)
  (params (bSubscribed :type Boolean) (TwitchSubscription :type Twitch%20Subscription%20Structure))
  (TwitchAuth|OnUserSubcribedtoChannel bSubscribed TwitchSubscription))

(event OnAuthenticationPageLoaded(TwitchAuth)
  (Widget|SetVisibility (Variables|Widgets|GetWebBrowser) "Visible")
  (Input|EnableCursor true))

(event OnAccessTokenPageLoaded(TwitchAuth)
  (Widget|SetVisibility (Variables|Widgets|GetWebBrowser) "Hidden")
  (Input|EnableCursor false))

(event EventBeginPlay
  (Utilities|FlowControl|Sequence
    (:then_0
      (Persistance|LoadAccessToken))
    (:then_1
      (Widgets|InitAuthenticationWidgets)
      (Class|TwitchAuthComponent|Authenticate (Variables|Default|GetTwitchAuth) (Variables|Widgets|GetWebBrowser)))))

(fn ConstructionScript)

(fn OnUserAuthenticated
  (params (Authenticated :type Boolean))
  (if Authenticated
    (bind _output_get (Variables|TwitchAuth|SetTwitchUser (Class|TwitchAuthComponent|GetUser (Variables|Default|GetTwitchAuth))))
    (Logging|PrintUserAuthentication _output_get)
    (Widget|RemovefromParent (Variables|Widgets|GetPreAuthenticationWidget))
    (Widgets|CreatePostAuthenticationWidget)
    (Class|TwitchAuthComponent|IsUserSubscribedtoChannel (Variables|Default|GetTwitchAuth) (Variables|TwitchAuth|GetSubscriptionChannel))
    (Persistance|SaveAccessToken)
    (else
      (Logging|PrintTwitchError (Class|TwitchAuthComponent|GetLastError (Variables|Default|GetTwitchAuth)))
      (Class|TwitchAuthComponent|ClearAccessToken (Variables|Default|GetTwitchAuth))
      (Widgets|CreatePreAuthenticationWidget)
      (Class|TwitchAuthComponent|Authenticate (Variables|Default|GetTwitchAuth) (Variables|Widgets|GetWebBrowser)))))

(fn OnUserSubcribedtoChannel
  (params (Subscribed :type Boolean) (TwitchSubscription :type Twitch%20Subscription%20Structure))
  (Default|SetVerification (Variables|Widgets|GetPostAuthenticationWidget) Subscribed)
  (if Subscribed
    (bind _output_get (Variables|TwitchAuth|SetTwitchSubscription TwitchSubscription))
    (Logging|PrintSubscription _output_get)
    (else
      (Logging|PrintTwitchError (Class|TwitchAuthComponent|GetLastError (Variables|Default|GetTwitchAuth))))))

(fn EnableCursor
  (params (bEnable :type Boolean))
  (Variables|/Script/Engine.PlayerController|SetbShowMouseCursor (Game|GetPlayerController 0) bEnable))

(fn CreatePreAuthenticationWidget
  (if (Utilities|IsValid (Variables|Widgets|GetPreAuthenticationWidget))
    (Widget|RemovefromParent (Variables|Widgets|GetPreAuthenticationWidget)))
  (bind _returnvalue (UserInterface|CreateWidget "/TwitchAuth/UIExample/UMG/WBP_PreAuthenticationWidget.WBP_PreAuthenticationWidget_C" (Game|GetPlayerController 0)))
  (bind _output_get (Variables|Widgets|SetPreAuthenticationWidget _returnvalue))
  (Variables|Widgets|SetWebBrowser (Variables|/TwitchAuth/UIExample/UMG/WBP_PreAuthenticationWidget.WBP_PreAuthenticationWidget_C|GetWebBrowser_0 _output_get))
  (Widget|SetVisibility (Variables|/TwitchAuth/UIExample/UMG/WBP_PreAuthenticationWidget.WBP_PreAuthenticationWidget_C|GetWebBrowser_0 _output_get) "Hidden")
  (UserInterface|Viewport|AddtoViewport (Variables|Widgets|GetPreAuthenticationWidget) 0))

(fn CreatePostAuthenticationWidget
  (if (Utilities|IsValid (Variables|Widgets|GetPostAuthenticationWidget))
    (Widget|RemovefromParent (Variables|Widgets|GetPostAuthenticationWidget)))
  (bind _returnvalue (UserInterface|CreateWidget "/TwitchAuth/UIExample/UMG/WBP_PostAuthenticationWidget.WBP_PostAuthenticationWidget_C" (Game|GetPlayerController 0)))
  (bind _output_get (Variables|Widgets|SetPostAuthenticationWidget _returnvalue))
  (UserInterface|Viewport|AddtoViewport _output_get 0))

(fn SaveAccessToken
  (bind _returnvalue (SaveGame|CreateSaveGameObject "/TwitchAuth/UIExample/Blueprints/BP_SaveGame.BP_SaveGame_C"))
  (bind _output_get (Variables|Persistance|SetSaveGame _returnvalue))
  (Variables|/TwitchAuth/UIExample/Blueprints/BP_SaveGame.BP_SaveGame_C|SetTwitchAuthAccessToken _output_get (Class|TwitchAuthComponent|GetAccessToken (Variables|Default|GetTwitchAuth)))
  (SaveGame|SaveGametoSlot (Variables|Persistance|GetSaveGame) (Variables|/TwitchAuth/UIExample/Blueprints/BP_SaveGame.BP_SaveGame_C|GetSaveSlotName (Variables|Persistance|GetSaveGame))))

(fn LoadAccessToken
  (bind _returnvalue (SaveGame|CreateSaveGameObject "/TwitchAuth/UIExample/Blueprints/BP_SaveGame.BP_SaveGame_C"))
  (bind _output_get (Variables|Persistance|SetSaveGame _returnvalue))
  (bind _returnvalue_2 (SaveGame|LoadGamefromSlot (Variables|/TwitchAuth/UIExample/Blueprints/BP_SaveGame.BP_SaveGame_C|GetSaveSlotName _output_get)))
  (bind _asbp_save_game (Utilities|Casting|CastToBP_SaveGame _returnvalue_2))
  (bind _output_get_2 (Variables|Persistance|SetSaveGame _asbp_save_game))
  (Class|TwitchAuthComponent|SetAccessToken (Variables|Default|GetTwitchAuth) (Variables|/TwitchAuth/UIExample/Blueprints/BP_SaveGame.BP_SaveGame_C|GetTwitchAuthAccessToken _output_get_2)))

(fn PrintTwitchError
  (params (TwitchError :type Twitch%20Error%20Structure))
  (bind (_error _status _message) (Utilities|Struct|BreakTwitchError TwitchError))
  (Development|PrintString (Utilities|String|Append _error "(" (Utilities|String|ToString(Integer) _status) "): " _message) true true "(R=1.000000,G=0.082119,B=0.000000,A=1.000000)" 5.0))

(fn PrintUserAuthentication
  (params (TwitchUser :type Twitch%20User%20Structure))
  (Development|PrintString (Utilities|String|Append (.display_name (Utilities|Struct|BreakTwitchUser TwitchUser)) " just signed in!") true true "(R=0.160393,G=1.000000,B=0.000000,A=1.000000)"))

(fn PrintSubscription
  (params (TwitchSubscirption :type Twitch%20Subscription%20Structure))
  (Development|PrintString (Utilities|String|Append (.display_name (Utilities|Struct|BreakTwitchUser (Variables|TwitchAuth|GetTwitchUser))) " is subscribed to channel " (.name (Utilities|Struct|BreakTwitchChannel (.channel (Utilities|Struct|BreakTwitchSubscription TwitchSubscirption))))) true true "(R=0.250554,G=1.000000,B=0.000000,A=1.000000)"))

(fn InitAuthenticationWidgets
  (if (> (Utilities|String|Len (Class|TwitchAuthComponent|GetAccessToken (Variables|Default|GetTwitchAuth))) 0)
    (Widgets|CreatePostAuthenticationWidget)
    (else
      (Widgets|CreatePreAuthenticationWidget))))